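; BP_Trap is a spike trap world prop that damages the player while they stand in its collider.
; An overlap sets SpikesUp, then after a short delay plays the spike animation and applies damage to BP_Player.
; IsActive gates a cooldown that loops back to strike again until an end overlap clears SpikesUp.
; A non-player trigger fails the cast after IsActive is cleared, leaving the trap inactive.
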(event OnComponentBeginOverlap(collider)
  (params (OverlappedComponent :type Primitive%20Component%20Object%20Reference) (OtherActor :type Actor%20Object%20Reference) (OtherComp :type Primitive%20Component%20Object%20Reference) (OtherBodyIndex :type Integer) (bFromSweep :type Boolean) (SweepResult :type Hit%20Result%20Structure%20%28by%20ref%29))
  (bind _trap (Variables|Default|GetTrap))
  (bind _output_get (Variables|Default|SetSpikesUp true))
  (Utilities|FlowControl|Delay 0.2 :!label _label)
  (if (and (Variables|Default|GetSpikesUp) (Variables|Default|GetIsActive))
    (Variables|Default|SetIsActive false)
    (Components|Animation|PlayAnimation _trap "/Game/WorldProps/trap/SpikeTrap_HideAnimation_Anim.SpikeTrap_HideAnimation_Anim" false)
    (Transformation|SetRelativeRotation _trap "0.000000,0.000000,90.000000" false false)
    (if _output_get
      (bind _asbp_player (Utilities|Casting|CastToBP_Player OtherActor))
      (Game|Damage|ApplyDamage _asbp_player 1.0 0 0)
      (Utilities|FlowControl|Delay 2.3)
      (Variables|Default|SetIsActive true)
      (goto _label))))

(event Collision|EventActorEndOverlap
  (params (OtherActor :type Actor%20Object%20Reference))
  (Variables|Default|SetSpikesUp false))

(event EventBeginPlay
  (bind _trap (Variables|Default|GetTrap))
  (Components|Animation|PlayAnimation _trap "/Game/WorldProps/trap/SpikeTrap_HideAnimation_Anim.SpikeTrap_HideAnimation_Anim" false)
  (Transformation|SetRelativeRotation _trap "0.000000,0.000000,90.000000" false false))

(fn ConstructionScript)