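; BP_EndGame is a world trigger that ends the game with a win when the player overlaps it.
; On overlap it disables player input, spins the player's mesh half a turn and sets HasWin on ABP_Player to drive the animation.
; After a short delay it shows the Win_HUD widget and switches to UI-only input with the mouse cursor visible.
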(event Collision|EventActorBeginOverlap
  (params (OtherActor :type Actor%20Object%20Reference))
  (bind _returnvalue (Game|GetPlayerController 0))
  (bind _asbp_player (Utilities|Casting|CastToBP_Player OtherActor))
  (Input|DisableInput _asbp_player _returnvalue)
  (Transformation|AddWorldRotation (Variables|/Script/Engine.Character|GetMesh _asbp_player) "0.000000,180.000000,0.000000" false false)
  (bind _asabp_player (Utilities|Casting|CastToABP_Player (Components|SkeletalMesh|GetAnimInstance (Variables|/Script/Engine.Character|GetMesh _asbp_player))))
  (Variables|/Game/Character/Animation/Player/ABP_Player.ABP_Player_C|SetHasWin _asabp_player true)
  (Utilities|FlowControl|Delay 5.0)
  (bind _returnvalue_2 (UserInterface|CreateWidget "/Game/Menu/Win_HUD.Win_HUD_C"))
  (UserInterface|Viewport|AddtoViewport _returnvalue_2 0)
  (Variables|/Script/Engine.PlayerController|SetbShowMouseCursor _returnvalue true)
  (Input|SetInputModeUIOnly _returnvalue 0 "DoNotLock" false))

(fn ConstructionScript)