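; Boss enemy that chases the player on sight via PawnSensing and AI MoveTo, damaging them on contact.
; A falling player who overlaps it bounces upward and damages it instead, triggering timed invincibility with a flashing mesh.
; Surviving a hit sends it back to its spawn point, where it turns around and restores health after a delay.
; At zero health it drops a Heart and is destroyed.
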(event OnSeePawn(PawnSensing)
  (params (Pawn :type Pawn%20Object%20Reference))
  ;[1 1 1] Detect and move to the player
  (Variables|Default|SetIsSeeingPlayer true)
  (CallFunction|FollowPlayer))

(event Custom|FollowPlayer
  ;[1 1 1] Detect and move to the player
  (if (Variables|Default|GetIsSeeingPlayer)
    (AI|AIMoveTo self "0, 0, 0" (Game|GetPlayerCharacter 0) 5.0 false)))

(event Collision|EventActorBeginOverlap
  (params (OtherActor :type Actor%20Object%20Reference))
  ;[1 1 1] Enemt take damage if the player jump on him
  (bind _asbp_player (Utilities|Casting|CastToBP_Player OtherActor))
  (if (AI|Components|NavMovement|IsFalling (Variables|/Script/Engine.Character|GetCharacterMovement _asbp_player))
    (Components|Movement|StopMovementImmediately (Variables|/Script/Engine.Character|GetCharacterMovement _asbp_player))
    (Character|LaunchCharacter _asbp_player (* (Math|Vector|GetUpVector (Variables|Default|GetHead)) (Math|Conversions|ToVector(Float) 1.25e+03)) false false)
    (Game|Damage|ApplyDamage self 1.0 0 0)
    (else
      (Game|Damage|ApplyDamage _asbp_player 1.0 0 0))))

(event EventTick
  (params (DeltaSeconds :type Float%20%28single-precision%29))
  (bind _mesh (Variables|Character|GetMesh))
  ;[1 1 1] Manage Damage and Invicibilty
  ;;[1 1 1] Manage Invicibility Frame and Flashing
  (if (not (Variables|Default|GetCanTakeDamage))
    (bind _output_get (Variables|Default|SetDamageTimer (- (Variables|Default|GetDamageTimer) DeltaSeconds)))
    (if (<= _output_get 0.0)
      (Rendering|SetVisibility _mesh true true)
      (Variables|Default|SetCanTakeDamage true)
      (Variables|Default|SetDamageTimer 2.0)
      (elif (< (Math|Float|%(Float) _output_get 0.2) 0.1)
        (Rendering|SetVisibility _mesh true true)
        (else
          (Rendering|SetVisibility _mesh false true))))))

(event Game|Damage|EventAnyDamage
  (params (Damage :type Float%20%28single-precision%29) (DamageType :type Damage%20Type%20Object%20Reference) (InstigatedBy :type Controller%20Object%20Reference) (DamageCauser :type Actor%20Object%20Reference))
  ;[1 1 1] Manage Damage and Invicibilty
  ;;[1 1 1] Manage Damage and Return to Base
  (if (Variables|Default|GetCanTakeDamage)
    (Variables|Default|SetCanTakeDamage false)
    (bind _output_get (Variables|Default|SetHealth (- (Variables|Default|GetHealth) Damage)))
    (if (<= _output_get 0.0)
      (Game|SpawnActorfromClass "/Game/WorldProps/Heart.Heart_C" (Transformation|GetActorTransform) "Undefined" "MultiplyWithRoot" 0 0)
      (Actor|DestroyActor)
      (else
        (Variables|Default|SetIsSeeingPlayer false)
        (AI|AIMoveTo self (Variables|Default|GetSpawn) 0 1e+01 false
          (:OnSuccess
            (Transformation|AddActorLocalRotation "0.000000,180.000000,0.000000" false false)
            (Utilities|FlowControl|Delay 5.0)
            (Variables|Default|SetHealth 2.0)))))))

(event EventBeginPlay
  ;[1 1 1] Init Spawn
  (Variables|Default|SetSpawn (Transformation|GetActorLocation)))

(fn ConstructionScript)