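; BP_Enemy is an enemy that chases the player and can be stomped.
; PawnSensing sightings set a seeing flag, never cleared here, and issue an AI MoveTo toward the player character.
; Overlapping a falling BP_Player stops their movement, launches them along the Head component's up vector, spawns a Heart and destroys the enemy.
; Any other BP_Player overlap applies damage to the player.
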(event OnSeePawn(PawnSensing)
  (params (Pawn :type Pawn%20Object%20Reference))
  ;[1 1 1] Detect and move to the player
  (Variables|Default|SetIsSeeingPlayer true)
  (CallFunction|FollowPlayer))

(event Custom|FollowPlayer
  ;[1 1 1] Detect and move to the player
  (if (Variables|Default|GetIsSeeingPlayer)
    (AI|AIMoveTo self "0, 0, 0" (Game|GetPlayerCharacter 0) 5.0 false)))

(event Collision|EventActorBeginOverlap
  (params (OtherActor :type Actor%20Object%20Reference))
  ;[1 1 1] Manage Damage
  (bind _asbp_player (Utilities|Casting|CastToBP_Player OtherActor))
  (if (AI|Components|NavMovement|IsFalling (Variables|/Script/Engine.Character|GetCharacterMovement _asbp_player))
    (Components|Movement|StopMovementImmediately (Variables|/Script/Engine.Character|GetCharacterMovement _asbp_player))
    (Character|LaunchCharacter _asbp_player (* (Math|Vector|GetUpVector (Variables|Default|GetHead)) (Math|Conversions|ToVector(Float) 7.5e+02)) false false)
    (Game|SpawnActorfromClass "/Game/WorldProps/Heart.Heart_C" (Transformation|GetActorTransform) "Undefined" "MultiplyWithRoot" 0 0)
    (Actor|DestroyActor)
    (else
      (Game|Damage|ApplyDamage _asbp_player 1.0 0 0))))

(fn ConstructionScript)